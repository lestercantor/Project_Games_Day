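; SaveGame_Settings is a save game object that stores the player's audio and input settings for the pause menu.
; It holds per-channel volumes for master, effects, music, UI, voice and input, plus a background-sound toggle and mouse sensitivity.
; FInitSave writes the default values, and FLoadSave returns all stored values at once, exposing the background-sound flag as SoundEnabled.
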(fn FInitSave
  (Variables|Default|SetMasterVolume 0.5)
  (Variables|Default|SetEffectsVolume 0.5)
  (Variables|Default|SetMusicVolume 0.5)
  (Variables|Default|SetUIVolume 0.5)
  (Variables|Default|SetVoiceVolume 1.0)
  (Variables|Default|SetSoundInBackground false)
  (Variables|Default|SetMouseSensitivity 1.0)
  (Variables|Default|SetInputVolume 1.0))

(fn FLoadSave
  (return (Variables|Default|GetMasterVolume) (Variables|Default|GetEffectsVolume) (Variables|Default|GetMusicVolume) (Variables|Default|GetUIVolume) (Variables|Default|GetVoiceVolume) (Variables|Default|GetSoundInBackground) (Variables|Default|GetMouseSensitivity) (Variables|Default|GetInputVolume)))