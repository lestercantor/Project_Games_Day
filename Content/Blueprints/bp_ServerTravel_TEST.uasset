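; Test trigger actor that moves a multiplayer session to another level when a player walks into it.
; When the first local player's pawn overlaps the Box, it gets bpGameMode_GamesDay and, if the pawn has authority, calls TravelTo with the TravelTest level.
; Otherwise it only prints a client message, though the game mode cast runs first, so that branch likely never fires on clients.
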(event OnComponentBeginOverlap(Box)
  (params (OverlappedComponent :type Primitive%20Component%20Object%20Reference) (OtherActor :type Actor%20Object%20Reference) (OtherComp :type Primitive%20Component%20Object%20Reference) (OtherBodyIndex :type Integer) (bFromSweep :type Boolean) (SweepResult :type Hit%20Result%20Structure%20%28by%20ref%29))
  (if (== OtherActor (Pawn|GetControlledPawn (Game|GetPlayerController 0)))
    (bind _asbp_game_mode_games_day (Utilities|Casting|CastTobpGameMode_GamesDay (Game|GetGameMode)))
    (if (Ability|HasAuthority OtherActor)
      (Development|PrintString "Host has travelled to next level")
      (Default|Travelto _asbp_game_mode_games_day "TravelTest")
      (else
        (Development|PrintString "Client trying to travel to next level")))))

(event EventBeginPlay)

(event Collision|EventActorBeginOverlap
  (params (OtherActor :type Actor%20Object%20Reference)))

(event EventTick
  (params (DeltaSeconds :type Float%20%28single-precision%29)))

(fn ConstructionScript)