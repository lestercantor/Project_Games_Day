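; Interactable wall poster prop in the lobby that opens a full-screen poster UI when the player interacts with it.
; Interact plays a paper sound, creates and shows the WallPoster widget, then switches the first player controller to UI-only input with the mouse cursor visible.
; SetFocus toggles custom depth rendering on the Poster mesh for highlighting and returns the poster's Name.
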(event EventInteract
  (params (InteractingActor :type Actor%20Object%20Reference))
  (bind _returnvalue (Game|GetPlayerController 0))
  (Audio|PlaySound2D "/Game/Blueprints/Sounds/Sound_UI/PaperUICue.PaperUICue" 1.0 1.0 0.0 0 0)
  (bind _returnvalue_2 (UserInterface|CreateWidget "/Game/Blueprints/All_Lobby_Assets/WallPoster/WallPosterWidget.WallPosterWidget_C"))
  (UserInterface|Viewport|AddtoViewport _returnvalue_2 0)
  (Input|SetInputModeUIOnly _returnvalue _returnvalue_2 "DoNotLock" false)
  (Variables|/Script/Engine.PlayerController|SetbShowMouseCursor _returnvalue true))

(fn ConstructionScript)

(fn SetFocus
  (params (Focus :type Boolean))
  (Rendering|SetRenderCustomDepth (Variables|Default|GetPoster) Focus)
  (return (Variables|Default|GetName)))