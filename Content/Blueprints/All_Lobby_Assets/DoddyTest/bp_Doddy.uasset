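; bp_Doddy is an interactable lobby actor with a dialogue screen and a speech bubble.
; Interact locks movement, blends the view to its camera, then opens the DoddyTextWidget with UI-only input and cursor.
; A server event multicasts the bubble, which shows, calls the fade-out on its Evildoddytext widget and hides after a short delay.
; SetFocus toggles the mesh's custom-depth highlight and returns the actor's Name.
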(event Custom|Server_ShowBubble
  (CallFunction|MulticastShowBubble))

(event Custom|Multicast_ShowBubble
  (Rendering|SetVisibility (Variables|Default|GetSpeechBubble) true false)
  (bind _asevildoddytext (Utilities|Casting|CastToEvildoddytext (UserInterface|GetWidget (Variables|Default|GetSpeechBubble))))
  (Default|FFadeOut _asevildoddytext)
  (Utilities|FlowControl|Delay 1.5)
  (Rendering|SetVisibility (Variables|Default|GetSpeechBubble) false false))

(event EventInteract
  (params (InteractingActor :type Actor%20Object%20Reference))
  (bind _returnvalue (Game|GetPlayerController 0))
  (Input|SetIgnoreMoveInput (Game|GetPlayerController 0) true)
  (Game|Player|SetViewTargetwithBlend (Game|GetPlayerController 0) (Components|GetOwner (Variables|Default|GetCamera)) 1.0 "VTBlend_Linear" 1.0 true)
  (Utilities|FlowControl|Delay 1.0)
  (bind _returnvalue_2 (UserInterface|CreateWidget "/Game/Blueprints/All_Lobby_Assets/DoddyTest/DoddyTextWidget.DoddyTextWidget_C" (Game|GetPlayerController 0)))
  (UserInterface|Viewport|AddtoViewport _returnvalue_2 0)
  (Input|SetInputModeUIOnly _returnvalue 0 "DoNotLock" false)
  (Variables|/Script/Engine.PlayerController|SetbShowMouseCursor _returnvalue true))

(fn ConstructionScript)

(fn SetFocus
  (params (Focus :type Boolean))
  (Rendering|SetRenderCustomDepth (Variables|Default|GetMesh) Focus)
  (return (Variables|Default|GetName)))