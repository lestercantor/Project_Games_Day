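; Lobby player character that picks up basketballs and throws them with a hold-to-charge shot.
; Pickup hides the attached ball actor and shows first- and third-person stand-in meshes.
; Holding Enhanced Input shoot builds client strength toward a randomized cap; release sends it to server events, which destroy the held ball and launch a spawned one along the camera's aim.
; Each shot also records scoring eligibility and three-point range on the player state.
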(event Custom|ServerSpawnItem
  (params (SpawnTransform :type Transform))
  ;[0.2427 0.25 0.06479] Server event to handle throwing the ball by giving it a velocity
  (CallFunction|FHideBasketball)
  (bind _returnvalue (Game|SpawnActorfromClass "/Game/Blueprints/All_Lobby_Assets/BP_Basketball/bp_BasketballToThrow.bp_BasketballToThrow_C" SpawnTransform "Undefined" "OverrideRootScale" (Components|GetOwner) 0))
  (Physics|SetPhysicsLinearVelocity (Variables|/Game/Blueprints/All_Lobby_Assets/BP_Basketball/bp_BasketballToThrow.bp_BasketballToThrow_C|GetMESH_Basketball _returnvalue) (* (Math|Vector|GetUnitDirection(Vector) (Transformation|GetWorldLocation (Variables|Default|GetFirstPersonCamera)) (Transformation|GetActorLocation _returnvalue)) (Variables|Default|GetServerThrowStrength)) true "None")
  (Development|PrintString "kobe" true true "(R=0.000000,G=0.106735,B=1.000000,A=1.000000)" 3.0)
  (CallFunction|ServerSoundatPlayer "/Game/Blueprints/Sounds/Sound_Effects/ThrowSFX_Cue.ThrowSFX_Cue" (Transformation|GetWorldLocation (Variables|Default|GetCapsuleComponent)) 0.5))

(event Custom|Server_SetThrowStrength
  (params (ServerThrowStrength :type Float%20%28single-precision%29))
  ;[1 0.4583 0.4583] Server events to increase the throw strength and to reset it after the ball has been thrown
  (Variables|Default|SetServerThrowStrength ServerThrowStrength))

(event Custom|Server_ScoreWhenShot
  ;[1 0.3931 0.9046] Server event to check if the current player is within or outside the 3 point line to determine how much score they will get
  (bind _asbp_player_state_games_day (Utilities|Casting|CastTobpPlayerState_GamesDay (Variables|Default|GetPlayerState)))
  (if (Variables|/Game/Blueprints/bpPlayerState_GamesDay.bpPlayerState_GamesDay_C|GetCanScore? _asbp_player_state_games_day)
    (Variables|/Game/Blueprints/bpPlayerState_GamesDay.bpPlayerState_GamesDay_C|SetCanScoreWhenShot? _asbp_player_state_games_day true)
    (if (Variables|/Game/Blueprints/bpPlayerState_GamesDay.bpPlayerState_GamesDay_C|GetIsLongRange? _asbp_player_state_games_day)
      (Variables|/Game/Blueprints/bpPlayerState_GamesDay.bpPlayerState_GamesDay_C|SetLongRangeWhenShot? _asbp_player_state_games_day true)
      (else
        (Variables|/Game/Blueprints/bpPlayerState_GamesDay.bpPlayerState_GamesDay_C|SetLongRangeWhenShot? _asbp_player_state_games_day false)))
    (else
      (Variables|/Game/Blueprints/bpPlayerState_GamesDay.bpPlayerState_GamesDay_C|SetCanScoreWhenShot? _asbp_player_state_games_day false))))

(event Custom|ResetThrow
  ;[1 0.4583 0.4583] Server events to increase the throw strength and to reset it after the ball has been thrown
  (Variables|Default|SetClientStrength (Math|Random|RandomFloatinRange 3.5e+02 4.5e+02)))

(event Custom|Client_SetThrowStrength
  ;[1 0.4583 0.4583] Server events to increase the throw strength and to reset it after the ball has been thrown
  (Variables|Default|SetClientStrength (Math|Float|Clamp(Float) (+ (Variables|Default|GetClientStrength) 13.0) (Variables|Default|GetClientStrength) (Math|Random|RandomFloatinRange 1e+03 1.2e+03))))

(event Input|EnhancedActionEvents|EnhancedInputActionIA_Shoot
  (params (ActionValue :type Boolean) (ElapsedSeconds :type Float%20%28double-precision%29) (TriggeredSeconds :type Float%20%28double-precision%29) (InputAction :type Input%20Action%20Object%20Reference :default "/Game/Blueprints/FirstPerson/Input/Actions/IA_Shoot.IA_Shoot"))
  (bind _firstpersoncamera (Variables|Default|GetFirstPersonCamera))
  ;[0.3854 0.1646 0.3132] Logic for shooting the ball using ue5 enhanced input
  (:Triggered
    (bind _isvalid (CallFunction|FHoldingSomething?))
    (if _isvalid
      (Utilities|FlowControl|Delay (/ 1.0 45.0))
      (CallFunction|ClientSetThrowStrength)))
  (:Completed
    (bind _isvalid_2 (CallFunction|FHoldingSomething?))
    (if _isvalid_2
      (CallFunction|ServerSetThrowStrength (Variables|Default|GetClientStrength))
      (CallFunction|ServerSpawnItem (Math|Transform|MakeTransform (+ (Transformation|GetWorldLocation _firstpersoncamera) (* (Math|Vector|GetForwardVector _firstpersoncamera) 8e+01)) "0, 0, 0" "1.000000,1.000000,1.000000"))
      (CallFunction|ResetThrow)
      (CallFunction|ServerScorewhenShot))))

(event EventBeginPlay
  (|CallParentFunction) ; This node is disabled and will not be called.\nDrag off pins to build functionality.
)

(event Collision|EventActorBeginOverlap
  (params (OtherActor :type Actor%20Object%20Reference)))

(event EventHandlePickup
  (params (ActorToAttach :type Actor%20Object%20Reference))
  (Variables|Default|SetActorToHold_REF ActorToAttach)
  (CallFunction|FShowBasketball))

(event EventTick
  (params (DeltaSeconds :type Float%20%28single-precision%29))
  (|CallParentFunction DeltaSeconds) ; This node is disabled and will not be called.\nDrag off pins to build functionality.
)

(event Input|KeyboardEvents|Tab
  (params (Key :type Key%20Structure))
  (:Pressed
    (Development|PrintString "lobby")))

(fn ConstructionScript
  (|CallParentFunction))

(fn FHideBasketball
  (bind _sm_basketballsocketthirdperson (Variables|Default|GetSM_BasketballSocketTHIRDPERSON))
  (bind _actortohold_ref (Variables|Default|GetActorToHold_REF))
  (Transformation|DetachFromActor _actortohold_ref "KeepRelative" "KeepRelative" "KeepRelative")
  (Actor|DestroyActor _actortohold_ref)
  (Components|StaticMesh|SetStaticMesh _sm_basketballsocketthirdperson 0)
  (Rendering|SetVisibility _sm_basketballsocketthirdperson false false)
  (Rendering|SetVisibility (Variables|Default|GetSM_BasketballSocketFIRSTPERSON) false false))

(fn FShowBasketball
  (bind _sm_basketballsocketthirdperson (Variables|Default|GetSM_BasketballSocketTHIRDPERSON))
  (bind _actortohold_ref (Variables|Default|GetActorToHold_REF))
  ;[1 1 1] attach the actor reference to the player and set the static mesh for first and third person view
  (Transformation|AttachComponentToComponent (Variables|Default|GetActorToHold_REF) (Variables|Default|GetSM_BasketballSocketTHIRDPERSON) "None" "SnapToTarget" "SnapToTarget" "KeepRelative" true)
  (Rendering|SetActorHiddenInGame _actortohold_ref true)
  (Rendering|SetVisibility _sm_basketballsocketthirdperson true false)
  (Components|StaticMesh|SetStaticMesh _sm_basketballsocketthirdperson (Variables|/Script/Engine.StaticMeshComponent|GetStaticMesh (Actor|GetComponentbyClass _actortohold_ref "/Script/Engine.StaticMeshComponent")))
  (Rendering|SetVisibility (Variables|Default|GetSM_BasketballSocketFIRSTPERSON) true false))