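; Lobby basketball bag that hands out a new basketball to whoever interacts with it.
; Interact spawns the ball just above the bag and passes it straight to the interacting actor's pickup handler.
; SetFocus toggles custom depth on the bag mesh for highlighting and returns its name.
; The separate server and local interaction handlers are empty.
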(event EventInteract
  (params (InteractingActor :type Actor%20Object%20Reference))
  (bind _actortospawn (CallFunction|SpawnBall))
  (Class|BpInterfaceAttachComponent|HandlePickup(Message) InteractingActor _actortospawn))

(fn ConstructionScript)

(fn HandleInteractionServer
  (params (Player :type BP%20First%20Person%20Character%20Object%20Reference)))

(fn HandleInteractionLocal
  (params (Player :type BP%20First%20Person%20Character%20Object%20Reference)))

(fn SpawnBall
  (bind _returnvalue (Game|SpawnActorfromClass (Variables|Default|GetSpawnBasketball) (Math|Transform|MakeTransform (+ (Transformation|GetActorLocation) (* (Transformation|GetActorUpVector) 8e+01)) "0, 0, 0" "1.000000,1.000000,1.000000") "Undefined" "OverrideRootScale" 0 0))
  (return _returnvalue))

(fn SetFocus
  (params (Focus :type Boolean))
  (Rendering|SetRenderCustomDepth (Variables|Default|GetBag) Focus)
  (return (Variables|Default|GetName)))