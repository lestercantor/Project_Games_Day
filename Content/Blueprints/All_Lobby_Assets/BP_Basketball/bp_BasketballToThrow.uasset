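; Interactable lobby basketball actor that can be picked up and otherwise expires on a short lifespan set at BeginPlay.
; Interact spawns a Bp_BasketballToHold just above the ball, passes it to the interacting actor through HandlePickupMessage, then destroys itself.
; SetFocus toggles custom depth rendering on the basketball mesh to mark focus.
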(event EventInteract
  (params (InteractingActor :type Actor%20Object%20Reference))
  (bind _actortospawn (CallFunction|SpawnBall))
  (Class|BpInterfaceAttachComponent|HandlePickup(Message) InteractingActor _actortospawn)
  (Actor|DestroyActor))

(event EventBeginPlay
  (Actor|SetLifeSpan 5.0))

(fn ConstructionScript)

(fn SpawnBall
  (bind _returnvalue (Game|SpawnActorfromClass "/Game/Blueprints/All_Lobby_Assets/BP_Basketball/bp_BasketballToHold.bp_BasketballToHold_C" (Math|Transform|MakeTransform (+ (Transformation|GetActorLocation) (* (Transformation|GetActorUpVector) 8e+01)) "0, 0, 0" "1.000000,1.000000,1.000000") "Undefined" "OverrideRootScale" 0 0))
  (return _returnvalue))

(fn SetFocus
  (params (Focus :type Boolean))
  (Rendering|SetRenderCustomDepth (Variables|Default|GetMESH_Basketball) Focus)
  (return (Variables|Default|GetName)))