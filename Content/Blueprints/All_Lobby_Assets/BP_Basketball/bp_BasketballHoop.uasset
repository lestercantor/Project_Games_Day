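; Basketball hoop for the lobby that awards points to the player state of whoever threw the ball.
; Two stacked overlap triggers feed server-named checks: the first caches the thrower's player state and flags a downward pass, the second scores if the ball still falls.
; Scoring requires the player's can-score flag, with extra credit for long-range shots.
; Failed second checks clear the flag and make the ball ignore physics-body collisions.
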(event OnComponentBeginOverlap(FirstCollisionCheck)
  (params (OverlappedComponent :type Primitive%20Component%20Object%20Reference) (OtherActor :type Actor%20Object%20Reference) (OtherComp :type Primitive%20Component%20Object%20Reference) (OtherBodyIndex :type Integer) (bFromSweep :type Boolean) (SweepResult :type Hit%20Result%20Structure%20%28by%20ref%29))
  (CallFunction|ServerCheckFirstCollision OtherActor))

(event OnComponentBeginOverlap(SecondCollisionCheck)
  (params (OverlappedComponent :type Primitive%20Component%20Object%20Reference) (OtherActor :type Actor%20Object%20Reference) (OtherComp :type Primitive%20Component%20Object%20Reference) (OtherBodyIndex :type Integer) (bFromSweep :type Boolean) (SweepResult :type Hit%20Result%20Structure%20%28by%20ref%29))
  (CallFunction|ServerCheckSecondCollision OtherActor))

(event Custom|Server_CheckFirstCollision
  (params (OtherActor :type Actor%20Object%20Reference))
  (bind _asbp_basketball_to_throw (Utilities|Casting|CastTobp_BasketballToThrow OtherActor))
  (bind _asbp_player_controller_games_day (Utilities|Casting|CastTobpPlayerController_GamesDay (Components|GetOwner _asbp_basketball_to_throw)))
  (bind _asbp_player_state_games_day (Utilities|Casting|CastTobpPlayerState_GamesDay (Variables|/Script/Engine.Controller|GetPlayerState _asbp_player_controller_games_day)))
  (Variables|Default|SetOwningPlayerState _asbp_player_state_games_day)
  (if (Variables|/Game/Blueprints/bpPlayerState_GamesDay.bpPlayerState_GamesDay_C|GetCanScoreWhenShot? (Variables|Default|GetOwningPlayerState))
    (if (< (.Z (Math|Vector|BreakVector (Transformation|GetVelocity _asbp_basketball_to_throw))) 0.0)
      (Variables|Default|SetPassedFirstProperly? true)
      (else
        (Variables|Default|SetPassedFirstProperly? false :!label _label)))
    (else
      (goto _label))))

(event Custom|Server_CheckSecondCollision
  (params (OtherActor :type Actor%20Object%20Reference))
  (bind _owningplayerstate (Variables|Default|GetOwningPlayerState))
  (bind _asbp_basketball_to_throw (Utilities|Casting|CastTobp_BasketballToThrow OtherActor))
  (if (Variables|/Game/Blueprints/bpPlayerState_GamesDay.bpPlayerState_GamesDay_C|GetCanScoreWhenShot? (Variables|Default|GetOwningPlayerState))
    (if (Variables|Default|GetPassedFirstProperly?)
      (if (< (.Z (Math|Vector|BreakVector (Transformation|GetVelocity _asbp_basketball_to_throw))) 0.0)
        (Variables|Default|SetPassedFirstProperly? false)
        (if (Variables|/Game/Blueprints/bpPlayerState_GamesDay.bpPlayerState_GamesDay_C|GetLongRangeWhenShot? _owningplayerstate)
          (Variables|/Game/Blueprints/bpPlayerState_GamesDay.bpPlayerState_GamesDay_C|SetBasketballScore _owningplayerstate (+ (Variables|/Game/Blueprints/bpPlayerState_GamesDay.bpPlayerState_GamesDay_C|GetBasketballScore _owningplayerstate) 2))
          (else
            (Math|Integer|IncrementInt (Variables|/Game/Blueprints/bpPlayerState_GamesDay.bpPlayerState_GamesDay_C|GetBasketballScore _owningplayerstate))))
        (else
          (Collision|SetCollisionResponsetoChannel (Variables|/Game/Blueprints/All_Lobby_Assets/BP_Basketball/bp_BasketballToThrow.bp_BasketballToThrow_C|GetMESH_Basketball _asbp_basketball_to_throw) "ECC_PhysicsBody" "ECR_Ignore" :!label _label)
          (Variables|Default|SetPassedFirstProperly? false)))
      (else
        (goto _label)))
    (else
      (goto _label))))

(fn ConstructionScript)