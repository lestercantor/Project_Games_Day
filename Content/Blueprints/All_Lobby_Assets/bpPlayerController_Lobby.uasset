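; Lobby player controller that opens a wall poster UI and carries a test event for resetting lobby start state.
; CreateWallPoster blocks move input, plays a paper sound, shows the poster widget in UI-only input mode and centres the visible cursor.
; The test event clears the lobby game mode's ready and started flags and has the game state remove its widget.
; An alternative movement-disabling path through the custom movement component is left unconnected.
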(event Custom|CreateWallPoster
  (bind _self self)
  ;[1 1 1] stops the player from moving if they were moving while doing interacting
  (Input|SetIgnoreMoveInput true)
  (Audio|PlaySound2D "/Game/Blueprints/Sounds/Sound_UI/PaperUICue.PaperUICue" 1.0 1.0 0.0 0 0)
  (bind _returnvalue (UserInterface|CreateWidget "/Game/Blueprints/All_Lobby_Assets/WallPoster/WallPosterWidget.WallPosterWidget_C" self))
  (UserInterface|Viewport|AddtoViewport _returnvalue 0)
  (Input|SetInputModeUIOnly _self _returnvalue "DoNotLock" false)
  (Variables|/Script/Engine.PlayerController|SetbShowMouseCursor _self true)
  (CallFunction|CentreMouse self))

(event Custom|test
  (bind _asbp_game_mode_lobby (Utilities|Casting|CastTobpGameMode_Lobby (Game|GetGameMode)))
  (Variables|/Game/Blueprints/All_Lobby_Assets/bpGameMode_Lobby.bpGameMode_Lobby_C|SetAllPlayersReady _asbp_game_mode_lobby false)
  (bind _asbp_game_state_games_day (Utilities|Casting|CastTobpGameState_GamesDay (Game|GetGameState)))
  (Default|RemoveWidget _asbp_game_state_games_day)
  (Variables|/Game/Blueprints/All_Lobby_Assets/bpGameMode_Lobby.bpGameMode_Lobby_C|SetStarted _asbp_game_mode_lobby false))

(event EventBeginPlay
  (|CallParentFunction) ; This node is disabled and will not be called.\nDrag off pins to build functionality.
)

(event EventTick
  (params (DeltaSeconds :type Float%20%28single-precision%29)))

(fn ConstructionScript
  (|CallParentFunction))