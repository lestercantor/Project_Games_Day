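; Game mode for the Manhunt mode that tracks when all players have joined and can pick a random hunter.
; It caches the Manhunt game state on BeginPlay; new-player handling retries until that is valid, then compares PlayerArray with Players to set AllPlayersJoined.
; PickRandomHunter stores a random player controller as the game state's HunterOwner, but nothing here calls it.
; The post-join delay leads nowhere, and StartGameTimer is unwired.
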(event Custom|PickRandomHunter
  (bind _asbp_player_controller_manhunt (Utilities|Casting|CastTobpPlayerController_Manhunt (Utilities|Array|Get(acopy) (Variables|Default|GetPlayers) (Math|Random|RandomIntegerinRange 0 (- (Utilities|Array|Length (Variables|Default|GetPlayers)) 1)))))
  (bind _output_get (Variables|/Game/Blueprints/All_Manhunt_Assets/bpGameState_Manhunt.bpGameState_Manhunt_C|SetHunterOwner (Variables|Default|GetGameStateManhunt) _asbp_player_controller_manhunt))
  (Development|PrintString (Utilities|GetDisplayName _output_get)))

(event EventBeginPlay
  (|CallParentFunction)
  (bind _asbp_game_state_manhunt (Utilities|Casting|CastTobpGameState_Manhunt (Variables|Default|GetGameState_Base)))
  (Variables|Default|SetGameStateManhunt _asbp_game_state_manhunt))

(event EventHandleStartingNewPlayer
  (params (NewPlayer :type Player%20Controller%20Object%20Reference))
  (bind _gamestatemanhunt (Variables|Default|GetGameStateManhunt))
  (|CallParentFunction NewPlayer)
  (Utilities|IsValid _gamestatemanhunt :!label _label
    (:Is%20Valid
      (if (== (Utilities|Array|Length (Variables|/Script/Engine.GameStateBase|GetPlayerArray _gamestatemanhunt)) (Utilities|Array|Length (Variables|Default|GetPlayers)))
        (Development|PrintString "all players have joined")
        (bind _output_get (Variables|Default|SetAllPlayersJoined? true))
        (if _output_get
          ;[1 1 1] unfreeze players after all players have joined -> maybe do a countdown until the game starts. game timer starts after hunter is done i think
          (Utilities|FlowControl|Delay 1.0)
          (else
            (Development|PrintString "not all players have joined" :!label _label_2)
            (Variables|Default|SetAllPlayersJoined? false)))
        (else
          (goto _label_2))))
    (:Is%20Not%20Valid
      (Utilities|FlowControl|Delay 0.2)
      (goto _label))))

(event EventOnLogout
  (params (ExitingController :type Controller%20Object%20Reference))
  (|CallParentFunction ExitingController))

(fn ConstructionScript)