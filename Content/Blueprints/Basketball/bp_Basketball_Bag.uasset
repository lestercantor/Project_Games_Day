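; Basketball bag actor that grows by ten percent of its current scale each time a player interacts with it.
; Interact calls a server event, which runs an empty server handler, then multicasts to the local handler and prints a debug string.
; The local handler sets the Scale variable, whose RepNotify applies it to the Bag component.
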(event Custom|ServerInteract
  (params (Player :type BP%20First%20Person%20Character%20Object%20Reference))
  (CallFunction|HandleInteractionServer Player)
  (CallFunction|MulticastInteract Player))

(event Custom|MulticastInteract
  (params (Player :type BP%20First%20Person%20Character%20Object%20Reference))
  (CallFunction|HandleInteractionLocal Player)
  (Development|PrintString "Multicasting to all clients"))

(event EventInteract
  (params (Player :type BP%20First%20Person%20Character%20Object%20Reference))
  (CallFunction|ServerInteract Player))

(fn ConstructionScript)

(fn HandleInteractionServer
  (params (Player :type BP%20First%20Person%20Character%20Object%20Reference)))

(fn HandleInteractionLocal
  (params (Player :type BP%20First%20Person%20Character%20Object%20Reference))
  (Variables|Default|SetScale (* (Variables|/Script/Engine.SceneComponent|GetRelativeScale3D (Variables|Default|GetBag)) 1.1)))

(fn OnRepScale
  (Transformation|SetRelativeScale3D (Variables|Default|GetBag) (Variables|Default|GetScale)))