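; Game mode for GamesDay that places joining players in the level and handles server-side level travel.
; Each new GamesDay player controller is added to a Players list, then possesses a first-person character spawned at the PlayerStart looked up by its zero-based join index as name.
; TravelTo runs a servertravel console command, appending the level name directly with no added space.
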(event Custom|TravelTo
  (params (LevelName :type String))
  (Development|ExecuteConsoleCommand (Utilities|String|Append "servertravel " LevelName) 0))

(event EventBeginPlay)

(event EventTick
  (params (DeltaSeconds :type Float%20%28single-precision%29)))

(event EventHandleStartingNewPlayer
  (params (NewPlayer :type Player%20Controller%20Object%20Reference))
  (bind _asbp_player_controller_games_day (Utilities|Casting|CastTobpPlayerController_GamesDay NewPlayer))
  (Utilities|Array|Add (Variables|Default|GetPlayers) _asbp_player_controller_games_day)
  (bind _returnvalue (Game|SpawnActorfromClass "/Game/FirstPerson/Blueprints/BP_FirstPersonCharacter.BP_FirstPersonCharacter_C" (Transformation|GetActorTransform (Class|GameModeBase|FindPlayerStart 0 (Utilities|String|ToString(Integer) (- (Utilities|Array|Length (Variables|Default|GetPlayers)) 1)))) "Undefined" "MultiplyWithRoot" 0 0))
  (Pawn|Possess NewPlayer _returnvalue))

(fn ConstructionScript)